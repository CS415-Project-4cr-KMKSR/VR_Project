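; BP_VRButton is a one-shot interactive button that restores the VR player's health when pressed.
; BeginPlay caches the Button component's relative location, and the first overlap by a BP_PlayerVRPawn slides it inward along local Y using MoveComponentTo.
; The press then sets the pawn's Health to a fixed value and plays a 2D pickup sound.
; IsPressed blocks repeat presses and is never reset.
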(event OnComponentBeginOverlap(Button)
  (params (OverlappedComponent :type Primitive%20Component%20Object%20Reference) (OtherActor :type Actor%20Object%20Reference) (OtherComp :type Primitive%20Component%20Object%20Reference) (OtherBodyIndex :type Integer) (bFromSweep :type Boolean) (SweepResult :type Hit%20Result%20Structure%20%28by%20ref%29))
  (if (not (Variables|Default|GetIsPressed))
    (bind _asbp_player_vrpawn (Utilities|Casting|CastToBP_PlayerVRPawn OtherActor))
    (Variables|Default|SetIsPressed true)
    (Components|MoveComponentTo (Variables|Default|GetButton) (- (Variables|Default|GetButtonStart) "0.000000,30.000000,0.000000") "0, 0, 0" false false 0.1 false)
    (Variables|/Game/Characters/BP_PlayerVRPawn.BP_PlayerVRPawn_C|SetHealth _asbp_player_vrpawn 1e+02)
    (Audio|SpawnSound2D "/Game/ActualLevel/Health-pickup-sound-effect.Health-pickup-sound-effect" 1.0 1.0 0.0 0)))

(event EventBeginPlay
  (Variables|Default|SetButtonStart (Variables|/Script/Engine.SceneComponent|GetRelativeLocation (Variables|Default|GetButton))))

(event Collision|EventActorBeginOverlap
  (params (OtherActor :type Actor%20Object%20Reference)))

(event EventTick
  (params (DeltaSeconds :type Float%20%28single-precision%29)))

(fn ConstructionScript)