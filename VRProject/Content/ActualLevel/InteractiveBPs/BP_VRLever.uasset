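; VR lever that a motion controller grabs and pulls to slide a pair of doors apart.
; Grab stores the controller, and Release clears it only if it is the one holding the lever.
; While held, Tick finds the controller's pitch in the lever's yaw-offset local space, adds it to the current pitch and clamps it to a quarter turn.
; That angle also drives both doors' opposite X offsets.
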(event EventBeginPlay)

(event Collision|EventActorBeginOverlap
  (params (OtherActor :type Actor%20Object%20Reference)))

(event EventTick
  (params (DeltaSeconds :type Float%20%28single-precision%29))
  (bind _staticmesh (Variables|Default|GetStaticMesh))
  (bind _staticmesh_2 (Variables|Default|GetStaticMesh))
  (bind _returnvalue (Transformation|GetWorldTransform _staticmesh))
  (bind _motion_controller (Variables|Default|GetMotion%20Controller)
    (:then
      (Transformation|SetRelativeRotation _staticmesh_2 (Math|Rotator|MakeRotator 0.0 (Math|Float|Clamp(Float) (+ (.pitch (Variables|/Script/Engine.SceneComponent|GetRelativeRotation _staticmesh_2)) (.pitch (Math|Rotator|FindLookatRotation (Math|Vector|MakeVector 0.0 0.0 0.0) (.location (Math|Transform|MakeRelativeTransform (Transformation|GetWorldTransform _motion_controller) (Math|Transform|MakeTransform (.location _returnvalue) (Math|Rotator|CombineRotators (.rotation _returnvalue) "90.000000,0.000000,0.000000") (.scale _returnvalue))))))) 0.0 9e+01) 0.0) false false)
      (Transformation|SetRelativeLocation (Variables|Default|GetLeftDoor) (Math|Vector|MakeVector (/ (Math|Float|Clamp(Float) (+ (.pitch (Variables|/Script/Engine.SceneComponent|GetRelativeRotation _staticmesh_2)) (.pitch (Math|Rotator|FindLookatRotation (Math|Vector|MakeVector 0.0 0.0 0.0) (.location (Math|Transform|MakeRelativeTransform (Transformation|GetWorldTransform _motion_controller) (Math|Transform|MakeTransform (.location _returnvalue) (Math|Rotator|CombineRotators (.rotation _returnvalue) "90.000000,0.000000,0.000000") (.scale _returnvalue))))))) 0.0 9e+01) -2.0) 0.0 0.0) false false)
      (Transformation|SetRelativeLocation (Variables|Default|GetRightDoor) (Math|Vector|MakeVector (/ (Math|Float|Clamp(Float) (+ (.pitch (Variables|/Script/Engine.SceneComponent|GetRelativeRotation _staticmesh_2)) (.pitch (Math|Rotator|FindLookatRotation (Math|Vector|MakeVector 0.0 0.0 0.0) (.location (Math|Transform|MakeRelativeTransform (Transformation|GetWorldTransform _motion_controller) (Math|Transform|MakeTransform (.location _returnvalue) (Math|Rotator|CombineRotators (.rotation _returnvalue) "90.000000,0.000000,0.000000") (.scale _returnvalue))))))) 0.0 9e+01) 2.0) 0.0 0.0) false false))
    (:else)))

(event EventGrab
  (params (MotionController :type Motion%20Controller%20Component%20Object%20Reference))
  (Variables|Default|SetMotion%20Controller MotionController))

(event EventRelease
  (params (MotionController :type Motion%20Controller%20Component%20Object%20Reference))
  (if (== MotionController (Variables|Default|GetMotion%20Controller))
    (Variables|Default|SetMotion%20Controller 0)))

(fn ConstructionScript)