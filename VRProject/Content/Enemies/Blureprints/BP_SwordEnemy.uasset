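; BP_SwordEnemy is a melee enemy character that wanders, chases the player within a sensing radius, and returns toward its spawn point.
; Self-calling AIMoveTo events with delays form a polling state machine, switching between walk and run speeds using distance checks.
; Sword overlaps damage BP_PlayerVRPawn, then briefly disable sword collision as a hit cooldown.
; Incoming damage reduces health; death disables movement and capsule collision before delayed destruction.
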(event OnComponentBeginOverlap(EnemySword)
  (params (OverlappedComponent :type Primitive%20Component%20Object%20Reference) (OtherActor :type Actor%20Object%20Reference) (OtherComp :type Primitive%20Component%20Object%20Reference) (OtherBodyIndex :type Integer) (bFromSweep :type Boolean) (SweepResult :type Hit%20Result%20Structure%20%28by%20ref%29))
  (if (Utilities|ClassIsChildOf (Utilities|GetClass OtherActor) "/Game/Characters/BP_PlayerVRPawn.BP_PlayerVRPawn_C")
    (Game|Damage|ApplyDamage OtherActor 7.0 0 0)
    (Collision|SetCollisionEnabled OverlappedComponent "NoCollision")
    (Utilities|FlowControl|Delay 1.0)
    (Collision|SetCollisionEnabled OverlappedComponent "QueryAndPhysics")))

(event Custom|MoveBack
  (AI|AIMoveTo self (Variables|Default|GetSpawnLocation) 0 1e+02 true
    (:then
      (Utilities|FlowControl|Delay 0.2)
      (if (<= (Transformation|GetDistanceTo (Game|Player|GetPlayerPawn 0)) (Variables|Default|GetSensingRadius))
        (CallFunction|ChasePlayer)
        (elif (<= (Math|Vector|Distance(Vector) (Variables|Default|GetSpawnLocation) (Transformation|GetActorLocation)) 5e+02)
          (Variables|/Script/Engine.CharacterMovementComponent|SetMaxWalkSpeed (Variables|Character|GetCharacterMovement) (Variables|Default|GetWalkSpeed))
          (CallFunction|MovetoRandomLocation)
          (else
            (CallFunction|MoveBack)))))))

(event Custom|MoveToRandomLocation
  (bind _randomlocation (Class|NavigationSystemV1|GetRandomLocationinNavigableRadius (Transformation|GetActorLocation) 4e+03 0 0))
  (AI|AIMoveTo self _randomlocation 0 5.0 true
    (:then
      (Utilities|FlowControl|Delay 2.0)
      (if (<= (Transformation|GetDistanceTo (Game|Player|GetPlayerPawn 0)) (Variables|Default|GetSensingRadius))
        (Variables|/Script/Engine.CharacterMovementComponent|SetMaxWalkSpeed (Variables|Character|GetCharacterMovement) (Variables|Default|GetRunSpeed))
        (CallFunction|ChasePlayer)
        (elif (<= (Math|Vector|Distance(Vector) (Variables|Default|GetSpawnLocation) (Transformation|GetActorLocation)) 2.4e+03)
          (CallFunction|MovetoRandomLocation)
          (else
            (Variables|/Script/Engine.CharacterMovementComponent|SetMaxWalkSpeed (Variables|Character|GetCharacterMovement) (Variables|Default|GetRunSpeed))
            (CallFunction|MoveBack)))))))

(event Custom|ChasePlayer
  (AI|AIMoveTo self "0, 0, 0" (Game|Player|GetPlayerPawn 0) 5e+01 true
    (:then
      (Utilities|FlowControl|Delay 0.2)
      (if (<= (Transformation|GetDistanceTo (Game|Player|GetPlayerPawn 0)) (Variables|Default|GetSensingRadius))
        (CallFunction|ChasePlayer)
        (else
          (CallFunction|MoveBack))))))

(event EventBeginPlay
  (Variables|Default|SetSpawnLocation (Transformation|GetActorLocation))
  (Variables|/Script/Engine.CharacterMovementComponent|SetMaxWalkSpeed (Variables|Character|GetCharacterMovement) (Variables|Default|GetWalkSpeed))
  (CallFunction|MovetoRandomLocation))

(event Game|Damage|EventAnyDamage
  (params (Damage :type Float%20%28single-precision%29) (DamageType :type Damage%20Type%20Object%20Reference) (InstigatedBy :type Controller%20Object%20Reference) (DamageCauser :type Actor%20Object%20Reference))
  (Development|PrintString (Utilities|String|ToString(Float) Damage))
  (Variables|Default|SetHealth (- (Variables|Default|GetHealth) Damage))
  (if (<= (Variables|Default|GetHealth) 0.0)
    (Pawn|Components|CharacterMovement|DisableMovement (Variables|Character|GetCharacterMovement))
    (Collision|SetCollisionEnabled (Variables|Collision|GetCapsuleComponent) "NoCollision")
    (Utilities|FlowControl|Delay 4.0)
    (Actor|DestroyActor)))

(fn ConstructionScript)